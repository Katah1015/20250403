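; BP_MoveRect is a Blueprint that moves a Cube component on Tick, apparently meant to trace a rectangle in the XZ plane.
; A MoveType state machine steps the relative location by a fixed, frame-rate-dependent amount, switching direction at coordinate thresholds.
; Left and Down increment like Right and Up, so the cube drifts along +X after the first two legs.
; EventOverlap copies its IsStop argument into IsPlaying, which gates the movement.
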(event EventTick
  (params (DeltaSeconds :type Float%20%28single-precision%29))
  (if (Variables|Default|GetIsPlaying)
    (switch Utilities|FlowControl|Switch|SwitchonMoveType (Variables|Default|GetMoveType)
      (:NewEnumerator0
        (bind _output_get (Variables|Default|SetXLocation (+ (Variables|Default|GetXLocation) 1.0)))
        (Transformation|SetRelativeLocation (Variables|Default|GetCube) (Math|Vector|MakeVector _output_get 0.0 (Variables|Default|GetZLocation)) false false)
        (if (> (Variables|Default|GetXLocation) 5e+02)
          (Variables|Default|SetMoveType "NewEnumerator1")))
      (:NewEnumerator1
        (bind _output_get_2 (Variables|Default|SetZLocation (+ (Variables|Default|GetZLocation) 1.0)))
        (Transformation|SetRelativeLocation (Variables|Default|GetCube) (Math|Vector|MakeVector (Variables|Default|GetXLocation) 0.0 _output_get_2) false false)
        (if (> (Variables|Default|GetZLocation) 5e+02)
          (Variables|Default|SetMoveType "NewEnumerator2")))
      (:NewEnumerator2
        (bind _output_get_3 (Variables|Default|SetXLocation (+ (Variables|Default|GetXLocation) 1.0)))
        (Transformation|SetRelativeLocation (Variables|Default|GetCube) (Math|Vector|MakeVector _output_get_3 0.0 (Variables|Default|GetZLocation)) false false)
        (if (< (Variables|Default|GetXLocation) 0.0)
          (Variables|Default|SetMoveType "NewEnumerator3")))
      (:NewEnumerator3
        (bind _output_get_4 (Variables|Default|SetZLocation (+ (Variables|Default|GetZLocation) 1.0)))
        (Transformation|SetRelativeLocation (Variables|Default|GetCube) (Math|Vector|MakeVector (Variables|Default|GetXLocation) 0.0 _output_get_4) false false)
        (if (< (Variables|Default|GetZLocation) 0.0)
          (Variables|Default|SetMoveType "NewEnumerator0"))))))

(fn ConstructionScript)

(fn EventOverlap
  (params (IsStop :type Boolean))
  (bind _output_get (Variables|Default|SetIsPlaying IsStop))
  (return _output_get))