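; BP_Swtich is an overlap-triggered switch that signals a list of other actors.
; Its Cube component's begin and end overlap events loop over the Actors array and call EventOverlap through BPI_Overlap with true on enter and false on exit.
; The overlapping actor is not filtered, so every begin or end overlap sends the signal.
; The switch's own EventOverlap function is a stub that returns false.
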(event OnComponentBeginOverlap(Cube)
  (params (OverlappedComponent :type Primitive%20Component%20Object%20Reference) (OtherActor :type Actor%20Object%20Reference) (OtherComp :type Primitive%20Component%20Object%20Reference) (OtherBodyIndex :type Integer) (bFromSweep :type Boolean) (SweepResult :type Hit%20Result%20Structure%20%28by%20ref%29))
  (for _array_element (Variables|Default|GetActors)
    (bind _asbpi_overlap (Utilities|Casting|CastToBPI_Overlap _array_element))
    (Default|EventOverlap _asbpi_overlap true)))

(event OnComponentEndOverlap(Cube)
  (params (OverlappedComponent :type Primitive%20Component%20Object%20Reference) (OtherActor :type Actor%20Object%20Reference) (OtherComp :type Primitive%20Component%20Object%20Reference) (OtherBodyIndex :type Integer))
  (for _array_element (Variables|Default|GetActors)
    (bind _asbpi_overlap (Utilities|Casting|CastToBPI_Overlap _array_element))
    (Default|EventOverlap _asbpi_overlap false)))

(fn ConstructionScript)

(fn EventOverlap
  (params (IsStop :type Boolean))
  (return false))