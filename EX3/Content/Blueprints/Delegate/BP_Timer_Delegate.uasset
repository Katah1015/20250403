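; BP_Timer_Delegate is a timer driven by a Switch's overlap event dispatcher, showing elapsed time on the HUD.
; On BeginPlay it binds a delegate to the Switch, apparently BindSwitchOverlap, which copies IsBegin into IsStop.
; While IsStop is true, despite the name, Tick accumulates delta time and sends a zero-padded MM:SS string to BP_HUD's UpdateTime.
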(event EventBeginPlay
  (EventDispatchers|BindEventtoEventDispatcherOverlap (Variables|Default|GetSwitch) (EventDispatchers|CreateEvent :!event BindSwitchOverlap)))

(event EventTick
  (params (DeltaSeconds :type Float%20%28single-precision%29))
  (if (Variables|Default|GetIsStop)
    (bind _output_get (Variables|Default|SetTotalDeltaSeconds (+ DeltaSeconds (Variables|Default|GetTotalDeltaSeconds))))
    (bind _asbp_hud (Utilities|Casting|CastToBP_HUD (HUD|GetHUD (Game|GetPlayerController 0))))
    (Default|UpdateTime _asbp_hud (Utilities|String|Append (CallFunction|FloattoStr00 (/ _output_get 6e+01)) ":" (CallFunction|FloattoStr00 (Math|Float|%(Float) _output_get 6e+01))))))

(fn ConstructionScript)

(fn FloattoStr00
  (params (Float :type Float%20%28double-precision%29))
  (bind _returnvalue (Math|Float|Floor Float))
  (bind _returnvalue_2 (Utilities|String|ToString(Integer) _returnvalue))
  (if (< Float 1e+01)
    (return (Utilities|String|Append "0" _returnvalue_2))
    (else
      (return _returnvalue_2))))

(fn BindSwitchOverlap
  (params (IsBegin :type Boolean))
  (Variables|Default|SetIsStop IsBegin))