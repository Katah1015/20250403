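; BP_CountBox_Delegate is a counter box that shows how many times a referenced Switch has signalled an overlap begin.
; On BeginPlay it binds to the Switch's overlap event dispatcher, so the switch drives the count through a delegate.
; Each begin event increments the count, wrapping to zero after nine, and pushes it to the CountWidget.
; Tick turns the widget component toward the player camera horizontally by flattening Z in the look-at.
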(event EventBeginPlay
  (EventDispatchers|BindEventtoEventDispatcherOverlap (Variables|Default|GetSwitch) (EventDispatchers|CreateEvent :!event BindSwitchOverlap)))

(event EventTick
  (params (DeltaSeconds :type Float%20%28single-precision%29))
  (bind _returnvalue (Game|GetPlayerCameraManager 0))
  (bind _widget (Variables|Default|GetWidget))
  (bind _returnvalue_2 (Transformation|GetActorLocation _returnvalue))
  (bind _returnvalue_3 (Transformation|GetWorldLocation _widget))
  (Transformation|SetWorldRotation (Variables|Default|GetWidget) (Math|Rotator|FindLookatRotation (Math|Vector|MakeVector (.x _returnvalue_3) (.y _returnvalue_3) 0.0) (Math|Vector|MakeVector (.x _returnvalue_2) (.y _returnvalue_2) 0.0)) false false))

(fn ConstructionScript)

(fn BindSwitchOverlap
  (params (IsBegin :type Boolean))
  (if IsBegin
    (CallFunction|UpdateCount)
    (CallFunction|PrintCount)))

(fn UpdateCount
  (bind _output_get (Variables|Default|SetCount (+ (Variables|Default|GetCount) 1)))
  (if (> _output_get 9)
    (Variables|Default|SetCount 0)))

(fn PrintCount
  (bind _ascount_widget (Utilities|Casting|CastToCountWidget (UserInterface|GetWidget (Variables|Default|GetWidget))))
  (Default|UpdateCount _ascount_widget (Variables|Default|GetCount)))